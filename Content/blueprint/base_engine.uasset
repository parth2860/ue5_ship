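; Base engine Blueprint with a tank mesh and a text render, apparently an interactable engine prop.
; Its useengine event turns the tank mesh a further 90 degrees in yaw and makes the text visible.
; Nothing in this graph triggers that event: BeginPlay, overlap and Tick are empty.
; Unconnected leftover nodes would cache a ui_main_valve widget and call UseEngine through a resetting DoOnce with a delay.
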(event `self.ReceiveBeginPlay`)

(event `self.ReceiveActorBeginOverlap`
  (params (OtherActor :type "Actor Object Reference")))

(event `self.ReceiveTick`
  (params (DeltaSeconds :type "Float (single-precision)")))

(event `use engine`
  (bind _tank_mesh (`self.tank_mesh`))
  (bind (_relativerotation_roll _relativerotation_pitch _relativerotation_yaw) (`KismetMathLibrary.BreakRotator` (`SceneComponent.RelativeRotation` _tank_mesh)))
  (`SceneComponent.K2_SetRelativeRotation` _tank_mesh (`KismetMathLibrary.MakeRotator` 0.0 0.0 (+ _relativerotation_yaw 90.0)) false false)
  (`SceneComponent.SetVisibility` (`self.TextRender`) true false))

(fn `UserConstructionScript`)