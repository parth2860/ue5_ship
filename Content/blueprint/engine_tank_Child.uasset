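; Child variant of an engine tank actor, with fuel and valve functions inherited from its parent.
; On BeginPlay it runs the parent logic, then casts its widget component's user widget to ui_engine_valve and stores it as WidgetRef.
; Tick, the construction script, AddFuel and ValveMech only forward to the parent, so the widget binding is the only logic added here.
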(event `self.ReceiveBeginPlay`
  (`parent.ReceiveBeginPlay`)
  (bind _asui_engine_valve (cast `/Game/blueprint/ui/ui_engine_valve` (`WidgetComponent.GetUserWidgetObject` (`self.Widget`))))
  (set `self.widget_ref` _asui_engine_valve))

(event `self.ReceiveTick`
  (params (DeltaSeconds :type "Float (single-precision)"))
  (`parent.ReceiveTick` DeltaSeconds))

(fn `add_fuel`
  (params (`fuel add` :type "Float (double-precision)"))
  (`parent.add_fuel` `fuel add`))

(fn `UserConstructionScript`
  (`parent.UserConstructionScript`))

(fn `valve_mech`
  (params (`value add` :type "Float (double-precision)") (`value subtract` :type "Float (double-precision)") (Condition :type Boolean))
  (`parent.valve_mech` `value add` `value subtract` Condition))