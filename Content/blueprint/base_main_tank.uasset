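; Main fuel tank actor with an adjustable valve and a widget showing capacity and transfer rate while something overlaps its sphere.
; ValveMech raises or lowers the valve rate within limits and rotates the valve mesh.
; A Tick-driven DoOnce and Delay runs a transfer every second: at sufficient valve rate the tank fills, and above a fill threshold it also feeds Base_engine_tank without deducting its own fuel.
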(event `self.ReceiveBeginPlay`
  (bind _asui_main_valve (cast `/Game/blueprint/ui/ui_main_valve` (`WidgetComponent.GetUserWidgetObject` (`self.Widget`))))
  (set `self.widget_ref` _asui_main_valve))

(event `self.ReceiveTick`
  (params (DeltaSeconds :type "Float (single-precision)"))
  (`/Engine/EditorBlueprintResources/StandardMacros.DoOnce` false :!label _label
    (:`Completed`
      (`KismetSystemLibrary.Delay` 1.0)
      (`self.transfer_fuel`)
      (goto _label :!via `Reset`))))

(event `self.Sphere.OnComponentBeginOverlap`
  (params (OverlappedComponent :type "PrimitiveComponent Object Reference") (OtherActor :type "Actor Object Reference") (OtherComp :type "PrimitiveComponent Object Reference") (OtherBodyIndex :type Integer) (bFromSweep :type Boolean) (SweepResult :type "HitResult Structure (by ref)"))
  (`SceneComponent.SetVisibility` (`self.Widget`) true false)
  (`Widget.SetVisibility` (`self.widget_ref`) "Visible"))

(event `self.Sphere.OnComponentEndOverlap`
  (params (OverlappedComponent :type "PrimitiveComponent Object Reference") (OtherActor :type "Actor Object Reference") (OtherComp :type "PrimitiveComponent Object Reference") (OtherBodyIndex :type Integer))
  (`SceneComponent.SetVisibility` (`self.Widget`) false false)
  (`Widget.SetVisibility` (`self.widget_ref`) "Hidden"))

(event `transfer_fuel`
  (if (>= (`self.total_valve_rate`) 50.0)
    (`self.add_fuel` 5.0)
    (if (>= (`self.current amount`) 40.0)
      (bind _returnvalue (`GameplayStatics.GetActorOfClass` "/Game/blueprint/base_engine_tank.base_engine_tank_C"))
      (`/Game/blueprint/base_engine_tank.add_fuel` _returnvalue 5.0))))

(fn `add_fuel`
  (params (`fuel add` :type "Float (double-precision)"))
  (if (not (>= (`self.current amount`) (`self.total amount`)))
    (bind _output_get (set `self.current amount` (+ `fuel add` (`self.current amount`))))
    (`/Game/blueprint/ui/ui_main_valve.capacity bar` (`self.widget_ref`) _output_get)))

(fn `remove fuel`
  (params (fuel_remove :type "Float (double-precision)"))
  (if (<= (`self.current amount`) 0.0)
    (`KismetSystemLibrary.PrintString` "tank empty")
    (else
      (bind _output_get (set `self.current amount` (- (`self.current amount`) fuel_remove)))
      (`KismetSystemLibrary.PrintString` (`KismetStringLibrary.Conv_DoubleToString` _output_get))
      (`/Game/blueprint/ui/ui_main_valve.capacity bar` (`self.widget_ref`) _output_get))))

(fn `UserConstructionScript`)

(fn `valve_mech`
  (params (`value add` :type "Float (double-precision)") (`value subtract` :type "Float (double-precision)") (Condition :type Boolean))
  (bind _returnvalue (and (>= (`self.total_valve_rate`) -125.0) (<= (`self.total_valve_rate`) 125.0)))
  (if Condition
    (if _returnvalue
      (bind _output_get (set `self.total_valve_rate` (+ `value add` (`self.total_valve_rate`))))
      (`SceneComponent.K2_AddLocalRotation` (`self.valve`) (`KismetMathLibrary.MakeRotator` _output_get) false false)
      (`/Game/blueprint/ui/ui_main_valve.set _transfer rate` (`self.widget_ref`) _output_get))
    (elif _returnvalue
      (bind _output_get_2 (set `self.total_valve_rate` (- (`self.total_valve_rate`) `value subtract`)))
      (`SceneComponent.K2_AddLocalRotation` (`self.valve`) (`KismetMathLibrary.MakeRotator` _output_get_2) false false)
      (`/Game/blueprint/ui/ui_main_valve.set _transfer rate` (`self.widget_ref`) _output_get_2))))